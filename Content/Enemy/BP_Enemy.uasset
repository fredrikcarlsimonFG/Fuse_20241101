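; BP_Enemy is an enemy Blueprint that exposes a patrol route and an attack event.
; Attack is a temporary visual, showing the Sphere component for a short delay and then hiding it.
; GetPatrolRoute returns the PatrolRoute variable to callers.
; LineOfSight calls for line tracing and mesh building sit unconnected in the event graph and construction script, so they never run.
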(event Custom|Attack
  ;[1 0.3822 0.442] Temporary to show attack
  (Rendering|SetVisibility (Variables|Default|GetSphere) true false)
  (Utilities|FlowControl|Delay 1.0)
  (Rendering|SetVisibility (Variables|Default|GetSphere) false false))

(event EventBeginPlay)

(event Collision|EventActorBeginOverlap
  (params (OtherActor :type Actor%20Object%20Reference)))

(event EventTick
  (params (DeltaSeconds :type Float%20%28single-precision%29)))

(fn ConstructionScript)

(fn GetPatrolRoute
  (return (Variables|Default|GetPatrolRoute)))