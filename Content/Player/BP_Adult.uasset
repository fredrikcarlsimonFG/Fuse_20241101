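; BP_Adult is a player Character Blueprint with camera look, movement and jumping through Enhanced Input.
; BeginPlay adds the default mapping context; look input is scaled by CameraSensitivity, and movement follows the camera, with forward flattened to the horizontal plane.
; Tick updates IsJumping from vertical velocity while airborne: true rising, false descending.
; The jump input is labelled as a glide trigger too, but only starts and stops jumping.
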(event Custom|SetIsJumping
  (bind _charactermovement (Variables|Character|GetCharacterMovement))
  ;[1 1 1] Check if jumping
  (if (AI|Components|NavMovement|IsFalling _charactermovement)
    (Math|Float|CompareFloat (.z (Variables|/Script/Engine.MovementComponent|GetVelocity _charactermovement)) 0.0
      (:>
        (Variables|Other|SetIsJumping true))
      (:<
        (Variables|Other|SetIsJumping false)))))

(event Input|EnhancedActionEvents|EnhancedInputActionIA_Move
  (params (ActionValue :type Vector%202D%20Structure) (ElapsedSeconds :type Float%20%28double-precision%29) (TriggeredSeconds :type Float%20%28double-precision%29) (InputAction :type Input%20Action%20Object%20Reference :default "/Game/ThirdPerson/Input/Actions/IA_Move.IA_Move"))
  (bind _camera (Variables|Default|GetCamera))
  (bind _returnvalue (Math|Vector|GetForwardVector _camera))
  ;[1 1 1] Character movement
  (Pawn|Input|AddMovementInput (Math|Vector|Normalize (Math|Vector|MakeVector (.x _returnvalue) (.y _returnvalue) 0.0)) (.y ActionValue) true)
  (Pawn|Input|AddMovementInput (Math|Vector|GetRightVector (Variables|Default|GetCamera)) (.x ActionValue) false))

(event Input|EnhancedActionEvents|EnhancedInputActionIA_Look
  (params (ActionValue :type Vector%202D%20Structure) (ElapsedSeconds :type Float%20%28double-precision%29) (TriggeredSeconds :type Float%20%28double-precision%29) (InputAction :type Input%20Action%20Object%20Reference :default "/Game/ThirdPerson/Input/Actions/IA_Look.IA_Look"))
  (bind _camerasensitivity (Variables|Tweakables|GetCameraSensitivity))
  (bind _returnvalue (* ActionValue _camerasensitivity))
  (bind (_x _y) (Math|Vector2D|BreakVector2D _returnvalue))
  ;[1 1 1] Camera movement
  (Pawn|Input|AddControllerYawInput _x)
  (Pawn|Input|AddControllerPitchInput _y))

(event Input|EnhancedActionEvents|EnhancedInputActionIA_Jump
  (params (ActionValue :type Boolean) (ElapsedSeconds :type Float%20%28double-precision%29) (TriggeredSeconds :type Float%20%28double-precision%29) (InputAction :type Input%20Action%20Object%20Reference :default "/Game/ThirdPerson/Input/Actions/IA_Jump.IA_Jump"))
  ;[1 1 1] Jump and Glide trigger
  (if ActionValue
    (Character|Jump)
    (else
      (Character|StopJumping))))

(event EventTick
  (params (DeltaSeconds :type Float%20%28single-precision%29))
  ;[1 1 1] Tick
  (CallFunction|SetIsJumping))

(event EventBeginPlay
  ;[1 1 1] Enable input
  (bind _asplayer_controller (Utilities|Casting|CastToPlayerController (Pawn|GetController)))
  (Input|AddMappingContext (PlayerController|LocalPlayerSubsystems|GetEnhancedInputLocalPlayerSubsystem _asplayer_controller) "/Game/ThirdPerson/Input/IMC_Default.IMC_Default" 0 "(bIgnoreAllPressedKeysUntilRelease=True,bForceImmediately=False,bNotifyUserSettings=False)"))

(fn ConstructionScript)