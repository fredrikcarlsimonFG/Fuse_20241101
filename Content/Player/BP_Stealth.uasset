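; BP_Stealth is a player-controlled stealth character that can hand control over to BP_Platformer.
; Enhanced Input drives camera look scaled by sensitivity and camera-relative movement, with forward motion flattened to the horizontal plane.
; The switch action blends the view to the first BP_Platformer found, waits out the blend, then possesses it.
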(event Input|EnhancedActionEvents|EnhancedInputActionIA_Move
  (params (ActionValue :type Vector%202D%20Structure) (ElapsedSeconds :type Float%20%28double-precision%29) (TriggeredSeconds :type Float%20%28double-precision%29) (InputAction :type Input%20Action%20Object%20Reference :default "/Game/ThirdPerson/Input/Actions/IA_Move.IA_Move"))
  (bind _camera (Variables|Default|GetCamera))
  (bind _returnvalue (Math|Vector|GetForwardVector _camera))
  ;[1 1 1] Character movement
  (Pawn|Input|AddMovementInput (Math|Vector|Normalize (Math|Vector|MakeVector (.x _returnvalue) (.y _returnvalue) 0.0)) (.y ActionValue) true)
  (Pawn|Input|AddMovementInput (Math|Vector|GetRightVector (Variables|Default|GetCamera)) (.x ActionValue) false))

(event Input|EnhancedActionEvents|EnhancedInputActionIA_Look
  (params (ActionValue :type Vector%202D%20Structure) (ElapsedSeconds :type Float%20%28double-precision%29) (TriggeredSeconds :type Float%20%28double-precision%29) (InputAction :type Input%20Action%20Object%20Reference :default "/Game/ThirdPerson/Input/Actions/IA_Look.IA_Look"))
  (bind _camerasensitivity (Variables|Default|GetCameraSensitivity))
  (bind _returnvalue (* ActionValue _camerasensitivity))
  (bind (_x _y) (Math|Vector2D|BreakVector2D _returnvalue))
  ;[1 1 1] Camera movement
  (Pawn|Input|AddControllerYawInput _x)
  (Pawn|Input|AddControllerPitchInput _y))

(event Input|EnhancedActionEvents|EnhancedInputActionIA_SwitchCharacter
  (params (ActionValue :type Boolean) (ElapsedSeconds :type Float%20%28double-precision%29) (TriggeredSeconds :type Float%20%28double-precision%29) (InputAction :type Input%20Action%20Object%20Reference :default "/Game/ThirdPerson/Input/Actions/IA_SwitchCharacter.IA_SwitchCharacter"))
  (bind _returnvalue (Game|GetPlayerController 0))
  ;[1 1 1] Switch character
  (:Triggered
    (bind _returnvalue_2 (Actor|GetActorOfClass "/Game/Player/BP_Platformer.BP_Platformer_C" :!label _label))
    (Game|Player|SetViewTargetwithBlend _returnvalue _returnvalue_2 (Variables|Default|GetCameraSwitchBlendTime) "VTBlend_Cubic" 0.0 true)
    (Utilities|FlowControl|Delay (Variables|Default|GetCameraSwitchBlendTime))
    (Pawn|Possess _returnvalue _returnvalue_2))
  (:Started
    (goto _label)))

(event EventBeginPlay
  ;[1 1 1] Enable input
  (bind _asplayer_controller (Utilities|Casting|CastToPlayerController (Pawn|GetController)))
  (Input|AddMappingContext (PlayerController|LocalPlayerSubsystems|GetEnhancedInputLocalPlayerSubsystem _asplayer_controller) "/Game/ThirdPerson/Input/IMC_Default.IMC_Default" 0 "(bIgnoreAllPressedKeysUntilRelease=True,bForceImmediately=False,bNotifyUserSettings=False)"))

(fn ConstructionScript)