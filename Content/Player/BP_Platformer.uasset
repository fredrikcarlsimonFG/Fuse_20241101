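; BP_Platformer is a player character with camera-relative movement, jumping and gliding, which can hand control to BP_Stealth when not falling.
; Holding jump past a retriggerable delay while airborne starts a glide that swaps gravity, speed and air control and damps velocity.
; Releasing jump cuts upward velocity, while Tick tracks jump state and refreshes the glide once on landing to restore defaults.
; Switching blends the camera before possessing the other character.
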(event Custom|Glide
  (bind _charactermovement (Variables|Character|GetCharacterMovement))
  ;[1 1 1] Glide
  (if (and (Variables|Other|GetIsHoldingSpace?) (AI|Components|NavMovement|IsFalling (Variables|Character|GetCharacterMovement)))
    (Variables|/Script/Engine.CharacterMovementComponent|SetGravityScale _charactermovement (Variables|Tweakables|GetGlideGravityScale))
    (Variables|/Script/Engine.CharacterMovementComponent|SetMaxWalkSpeed _charactermovement (Variables|Tweakables|GetGlideMoveSpeed))
    (Variables|/Script/Engine.CharacterMovementComponent|SetAirControl _charactermovement (Variables|Tweakables|GetGlideAirControl))
    (Variables|/Script/Engine.MovementComponent|SetVelocity _charactermovement (Math|Vector|MakeVector (.x (/ (Variables|/Script/Engine.MovementComponent|GetVelocity _charactermovement) "1.500000,1.500000,1.500000")) (.y (/ (Variables|/Script/Engine.MovementComponent|GetVelocity _charactermovement) "1.500000,1.500000,1.500000")) 0.0))
    (Variables|Other|SetIsGliding true)
    (else
      (Variables|/Script/Engine.CharacterMovementComponent|SetGravityScale _charactermovement (Variables|Other|GetGravity))
      (Variables|/Script/Engine.CharacterMovementComponent|SetMaxWalkSpeed _charactermovement (Variables|Other|GetDefaultMoveSpeed))
      (Variables|/Script/Engine.CharacterMovementComponent|SetAirControl _charactermovement (Variables|Other|GetDefaultAirControl))
      (Variables|Other|SetIsGliding false))))

(event Custom|SetIsJumping
  (bind _charactermovement (Variables|Character|GetCharacterMovement))
  ;[1 1 1] Check if jumping
  (if (AI|Components|NavMovement|IsFalling _charactermovement)
    (Math|Float|CompareFloat (.z (Variables|/Script/Engine.MovementComponent|GetVelocity _charactermovement)) 0.0
      (:>
        (Variables|Other|SetIsJumping true))
      (:<
        (Variables|Other|SetIsJumping false)))))

(event Custom|DisableGlide
  ;[1 1 1] Disable Glide when grounded
  (if (AI|Components|NavMovement|IsFalling (Variables|Character|GetCharacterMovement))
    (goto _label Reset)
    (else
      (Utilities|FlowControl|DoOnce false :!label _label
        (:Completed
          (CallFunction|Glide))))))

(event Input|EnhancedActionEvents|EnhancedInputActionIA_Move
  (params (ActionValue :type Vector%202D%20Structure) (ElapsedSeconds :type Float%20%28double-precision%29) (TriggeredSeconds :type Float%20%28double-precision%29) (InputAction :type Input%20Action%20Object%20Reference :default "/Game/ThirdPerson/Input/Actions/IA_Move.IA_Move"))
  (bind _camera (Variables|Default|GetCamera))
  (bind _returnvalue (Math|Vector|GetForwardVector _camera))
  ;[1 1 1] Character movement
  (:Triggered
    (Pawn|Input|AddMovementInput (Math|Vector|Normalize (Math|Vector|MakeVector (.x _returnvalue) (.y _returnvalue) 0.0)) (.y ActionValue) true)
    (Pawn|Input|AddMovementInput (Math|Vector|GetRightVector (Variables|Default|GetCamera)) (.x ActionValue) false))
  (:Started
    (Variables|Other|SetOnMove true)
    (Utilities|FlowControl|DelayUntilNextTick)
    (Variables|Other|SetOnMove false)))

(event Input|EnhancedActionEvents|EnhancedInputActionIA_Look
  (params (ActionValue :type Vector%202D%20Structure) (ElapsedSeconds :type Float%20%28double-precision%29) (TriggeredSeconds :type Float%20%28double-precision%29) (InputAction :type Input%20Action%20Object%20Reference :default "/Game/ThirdPerson/Input/Actions/IA_Look.IA_Look"))
  (bind _camerasensitivity (Variables|Tweakables|GetCameraSensitivity))
  (bind _returnvalue (* ActionValue _camerasensitivity))
  (bind (_x _y) (Math|Vector2D|BreakVector2D _returnvalue))
  ;[1 1 1] Camera movement
  (Pawn|Input|AddControllerYawInput _x)
  (Pawn|Input|AddControllerPitchInput _y))

(event Input|EnhancedActionEvents|EnhancedInputActionIA_SwitchCharacter
  (params (ActionValue :type Boolean) (ElapsedSeconds :type Float%20%28double-precision%29) (TriggeredSeconds :type Float%20%28double-precision%29) (InputAction :type Input%20Action%20Object%20Reference :default "/Game/ThirdPerson/Input/Actions/IA_SwitchCharacter.IA_SwitchCharacter"))
  (bind _returnvalue (Game|GetPlayerController 0))
  ;[1 1 1] Switch character
  (:Triggered
    (if (not (AI|Components|NavMovement|IsFalling (Variables|Character|GetCharacterMovement))) :!label _label
      (bind _returnvalue_2 (Actor|GetActorOfClass "/Game/Player/BP_Stealth.BP_Stealth_C"))
      (Game|Player|SetViewTargetwithBlend _returnvalue _returnvalue_2 (Variables|Tweakables|GetCameraSwitchBlendTime) "VTBlend_Cubic" 0.0 true)
      (Utilities|FlowControl|Delay (Variables|Tweakables|GetCameraSwitchBlendTime))
      (Pawn|Possess _returnvalue _returnvalue_2)))
  (:Started
    (goto _label)))

(event Input|EnhancedActionEvents|EnhancedInputActionIA_Jump
  (params (ActionValue :type Boolean) (ElapsedSeconds :type Float%20%28double-precision%29) (TriggeredSeconds :type Float%20%28double-precision%29) (InputAction :type Input%20Action%20Object%20Reference :default "/Game/ThirdPerson/Input/Actions/IA_Jump.IA_Jump"))
  (bind _charactermovement (Variables|Character|GetCharacterMovement))
  ;[1 1 1] Jump and Glide trigger
  (if ActionValue
    (Character|Jump)
    (bind _output_get (Variables|Other|SetIsHoldingSpace? true))
    (Utilities|FlowControl|RetriggerableDelay (Variables|Tweakables|GetGlideTriggerTime))
    (if _output_get
      (CallFunction|Glide))
    (else
      (Character|StopJumping)
      (Variables|Other|SetIsHoldingSpace? false)
      (CallFunction|Glide)
      (if (> (.z (Variables|/Script/Engine.MovementComponent|GetVelocity _charactermovement)) 0.0)
        (Variables|/Script/Engine.MovementComponent|SetVelocity _charactermovement (Math|Vector|MakeVector (.x (Variables|/Script/Engine.MovementComponent|GetVelocity _charactermovement)) (.y (Variables|/Script/Engine.MovementComponent|GetVelocity _charactermovement)) (/ (.z (Variables|/Script/Engine.MovementComponent|GetVelocity _charactermovement)) 4.0)))))))

(event EventTick
  (params (DeltaSeconds :type Float%20%28single-precision%29))
  ;[1 1 1] Tick
  (CallFunction|SetIsJumping)
  (if (Variables|Other|GetBeginPlayFinished)
    (CallFunction|DisableGlide)))

(event EventBeginPlay
  (bind _charactermovement (Variables|Character|GetCharacterMovement))
  ;[1 1 1] Enable input
  (bind _asplayer_controller (Utilities|Casting|CastToPlayerController (Pawn|GetController)))
  (Input|AddMappingContext (PlayerController|LocalPlayerSubsystems|GetEnhancedInputLocalPlayerSubsystem _asplayer_controller) "/Game/ThirdPerson/Input/IMC_Default.IMC_Default" 0 "(bIgnoreAllPressedKeysUntilRelease=True,bForceImmediately=False,bNotifyUserSettings=False)")
  ;[1 1 1] Set Standard variables
  (Variables|Other|SetGravity (Variables|/Script/Engine.CharacterMovementComponent|GetGravityScale _charactermovement))
  (Variables|Other|SetDefaultMoveSpeed (Variables|/Script/Engine.CharacterMovementComponent|GetMaxWalkSpeed _charactermovement))
  (Variables|Other|SetDefaultAirControl (Variables|/Script/Engine.CharacterMovementComponent|GetAirControl _charactermovement))
  (Variables|Other|SetBeginPlayFinished true))

(fn ConstructionScript)