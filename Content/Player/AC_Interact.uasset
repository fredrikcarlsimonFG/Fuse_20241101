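; AC_Interact is a player interaction component that lets the player rotate a nearby mirror.
; An InRangeOfMirror event stores the mirror reference and an in-range flag.
; While in range, temporary Q and E key bindings call RotateMirror on that mirror with opposite boolean directions.
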(event EventBeginPlay)

(event EventTick
  (params (DeltaSeconds :type Float%20%28single-precision%29)))

(event EventInRangeOfMirror
  (params (Reference :type BP%20Puzzle%20Mirror%20Object%20Reference) (inRange? :type Boolean))
  (Variables|MirrorPuzzle|SetMirrorRef Reference)
  (Variables|MirrorPuzzle|SetinRange inRange?))

(event Input|KeyboardEvents|Q
  (params (Key :type Key%20Structure :default "None"))
  ;[1 1 1] Temporary Controls
  (:Pressed
    (if (Variables|MirrorPuzzle|GetinRange)
      (Default|RotateMirror (Variables|MirrorPuzzle|GetMirrorRef) true))))

(event Input|KeyboardEvents|E
  (params (Key :type Key%20Structure :default "None"))
  ;[1 1 1] Temporary Controls
  (:Pressed
    (if (Variables|MirrorPuzzle|GetinRange)
      (Default|RotateMirror (Variables|MirrorPuzzle|GetMirrorRef) false))))