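; BP_Windthing_RotatingObject is a level design actor that spins its WindSpinner component around the local pitch axis, with gradual spin-up and spin-down.
; StartRotating and StopRotating toggle a flag that Tick reads to ramp the current speed toward RotationSpeed or back toward zero.
; The ramp scales with delta time and a multiplier, while the negative rotation step applied each tick depends only on current speed, so spin rate is frame-rate dependent.
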(event Custom|StartRotating
  (Variables|Default|SetbIsRotating true))

(event Custom|StopRotating
  (Variables|Default|SetbIsRotating false))

(event EventTick
  (params (DeltaSeconds :type Float%20%28single-precision%29))
  (Variables|Default|SetDelta%20Seconds DeltaSeconds)
  (Utilities|FlowControl|Sequence
    (:then_0
      (if (Variables|Default|GetbIsRotating)
        (Utilities|FlowControl|Sequence
          (:then_0
            (if (< (Variables|Default|GetCurrentRotationSpeed) (Variables|Default|GetRotationSpeed))
              (Variables|Default|SetCurrentRotationSpeed (+ (Variables|Default|GetCurrentRotationSpeed) (* (Variables|Default|GetDelta%20Seconds) (Variables|Default|GetSpeedStartEndMultiplier))))))
          (:then_1
            (Transformation|AddLocalRotation (Variables|Default|GetWindSpinner) (Math|Rotator|MakeRotator 0.0 (* (Variables|Default|GetCurrentRotationSpeed) -0.01) 0.0) false false :!label _label)))))
    (:then_1
      (if (and (> (Variables|Default|GetCurrentRotationSpeed) 0.0) (not (Variables|Default|GetbIsRotating)))
        (Variables|Default|SetCurrentRotationSpeed (- (Variables|Default|GetCurrentRotationSpeed) (* (Variables|Default|GetDelta%20Seconds) (Variables|Default|GetSpeedStartEndMultiplier))))
        (goto _label)))))

(fn ConstructionScript)