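; BP_HairDryer is a level-design hair dryer that switches wind-line particles and layered audio on and off through SpawnParticles and DisableParticles.
; BeginPlay spawns the loop sound muted and deactivates the particles.
; SpawnParticles restarts the effect, plays a start sound, then raises loop volume after a delay.
; DisableParticles sets a flag that Tick reads to mute the loop and play the end sound once via a resettable DoOnce.
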(event Custom|SpawnParticles
  (bind _windlines (Variables|Default|GetWindLines))
  (bind _staticmesh (Variables|Default|GetStaticMesh))
  (bind _returnvalue (Transformation|GetWorldLocation _staticmesh))
  (Variables|Default|SetShouldTurnOff false)
  (Niagara|ReinitializeSystem _windlines)
  (Components|Activation|SetActive _windlines true false)
  (Audio|PlaySoundatLocation "/Game/Audio/SFX/Hairdryer/Fuse_-_sfx_-_Hairdryer_Start.Fuse_-_sfx_-_Hairdryer_Start" _returnvalue "0, 0, 0" 1.0 1.0 0.0 0 0 0 0)
  (Utilities|FlowControl|Delay 1.0)
  (Audio|Components|Audio|SetVolumeMultiplier (Variables|Default|GetLoopSound) 1.0 :!class /Script/Engine.AudioComponent)
  (Utilities|FlowControl|DoOnce false) ; enters at Reset
)

(event Custom|DisableParticles
  (Variables|Default|SetShouldTurnOff true)
  (Components|Activation|SetActive (Variables|Default|GetWindLines) false false))

(event EventTick
  (params (DeltaSeconds :type Float%20%28single-precision%29))
  (if (Variables|Default|GetShouldTurnOff)
    (Audio|Components|Audio|SetVolumeMultiplier (Variables|Default|GetLoopSound) 0.0 :!class /Script/Engine.AudioComponent)
    (Utilities|FlowControl|DoOnce false
      (:Completed
        (Audio|PlaySoundatLocation "/Game/Audio/SFX/Hairdryer/Fuse_-_sfx_-_Hairdryer_End.Fuse_-_sfx_-_Hairdryer_End" (Transformation|GetWorldLocation (Variables|Default|GetStaticMesh)) "0, 0, 0" 1.0 1.0 0.0 0 0 0 0)))))

(event EventBeginPlay
  (bind _returnvalue (Audio|SpawnSoundatLocation "/Game/Audio/SFX/Hairdryer/Fuse_-_sfx_-_Hairdryer_Mid.Fuse_-_sfx_-_Hairdryer_Mid" (Transformation|GetWorldLocation (Variables|Default|GetStaticMesh)) "0, 0, 0" 1.0 1.0 0.0 0 0))
  (bind _output_get (Variables|Default|SetLoopSound _returnvalue))
  (Audio|Components|Audio|SetVolumeMultiplier _output_get 0.0 :!class /Script/Engine.AudioComponent)
  (Components|Activation|SetActive (Variables|Default|GetWindLines) false false))

(fn ConstructionScript)