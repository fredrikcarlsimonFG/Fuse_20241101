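; Puzzle mirror actor that rotates in yaw steps, with a prompt widget shown around player proximity.
; Overlap with BP_Platformer tells its ACInteract component whether the mirror is in range and drives a timeline that fades the widget's alpha.
; RotateMirror turns clockwise or counter-clockwise by RotationAmount through a timeline lerp, ignoring calls while already rotating.
; Each tick billboards the widget toward the player camera with pitch held at zero.
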(event OnComponentBeginOverlap(OverlapArea)
  (params (OverlappedComponent :type Primitive%20Component%20Object%20Reference) (OtherActor :type Actor%20Object%20Reference) (OtherComp :type Primitive%20Component%20Object%20Reference) (OtherBodyIndex :type Integer) (bFromSweep :type Boolean) (SweepResult :type Hit%20Result%20Structure%20%28by%20ref%29))
  (bind _asbp_platformer (Utilities|Casting|CastToBP_Platformer OtherActor))
  (Class|BPIInteract|InRangeOfMirror(Message) (Variables|/Game/Player/BP_Platformer.BP_Platformer_C|GetAC_Interact _asbp_platformer) self true)
  (if (> (Variables|Default|GetTimelineTime) 0.0)
    (bind _value (Timeline|Timeline Play)
      (:Update
        (bind _output_get (Variables|Default|SetTimelineTime _value))
        (Class|WidgetComponent|SetTintColorandOpacity (Variables|Default|GetWidget) (Utilities|Struct|MakeLinearColor 1.0 1.0 1.0 _output_get)))
      (:Finished
        (Variables|Default|SetTimelineTime 0.0)))
    (else
      (Timeline|Timeline PlayFromStart))))

(event OnComponentEndOverlap(OverlapArea)
  (params (OverlappedComponent :type Primitive%20Component%20Object%20Reference) (OtherActor :type Actor%20Object%20Reference) (OtherComp :type Primitive%20Component%20Object%20Reference) (OtherBodyIndex :type Integer))
  (bind _asbp_platformer (Utilities|Casting|CastToBP_Platformer OtherActor))
  (Class|BPIInteract|InRangeOfMirror(Message) (Variables|/Game/Player/BP_Platformer.BP_Platformer_C|GetAC_Interact _asbp_platformer) 0 false)
  (if (> (Variables|Default|GetTimelineTime) 0.0)
    (bind _value (Timeline|Timeline ReverseFromEnd)
      (:Update
        (bind _output_get (Variables|Default|SetTimelineTime _value))
        (Class|WidgetComponent|SetTintColorandOpacity (Variables|Default|GetWidget) (Utilities|Struct|MakeLinearColor 1.0 1.0 1.0 _output_get)))
      (:Finished
        (Variables|Default|SetTimelineTime 0.0)))
    (else
      (Timeline|Timeline Reverse))))

(event EventBeginPlay
  (Class|WidgetComponent|SetTintColorandOpacity (Variables|Default|GetWidget) (Utilities|Struct|MakeLinearColor 1.0 1.0 1.0 0.0)))

(event EventTick
  (params (DeltaSeconds :type Float%20%28single-precision%29))
  (CallFunction|RotateImage))

(event EventRotateMirror
  (params (Clockwise? :type Boolean))
  (bind _returnvalue (Transformation|GetActorRotation))
  (bind _rotation_amount (Variables|Default|GetRotation%20Amount))
  (if (not (Variables|Default|GetRotating))
    (Variables|Default|SetRotating true)
    (Variables|Default|SetCurrent%20Angle (.yaw _returnvalue))
    (Variables|Default|SetNew%20Angle (select Clockwise? (+ (.yaw _returnvalue) _rotation_amount) (- (.yaw _returnvalue) _rotation_amount)))
    (bind _rotation (Timeline|Rotate%20Mirror PlayFromStart)
      (:Update
        (Transformation|SetActorRotation (Math|Rotator|Lerp(Rotator) (Math|Rotator|MakeRotator 0.0 0.0 (Variables|Default|GetCurrent%20Angle)) (Math|Rotator|MakeRotator 0.0 0.0 (Variables|Default|GetNew%20Angle)) _rotation)))
      (:Finished
        (Variables|Default|SetRotating false)))))

(fn ConstructionScript)

(fn RotateImage
  (bind _returnvalue (Game|GetPlayerCameraManager 0))
  (bind _widget (Variables|Default|GetWidget))
  (bind _returnvalue_2 (Camera|GetCameraLocation _returnvalue))
  (bind _returnvalue_3 (Transformation|GetWorldLocation _widget))
  (bind _returnvalue_4 (Math|Rotator|FindLookatRotation _returnvalue_3 _returnvalue_2))
  (Transformation|SetWorldRotation (Variables|Default|GetWidget) (Math|Rotator|MakeRotator (.roll _returnvalue_4) 0.0 (.yaw _returnvalue_4)) false false))