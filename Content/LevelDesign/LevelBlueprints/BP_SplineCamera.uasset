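; Spline-driven cutscene camera actor that takes over the player's view on game start, trigger overlap or event.
; Tick runs one of three modes: automatic travel with optional look-at spline, a cable ride along another spline with a spark, or following the player's position along the spline.
; A curve scales travel speed, and player movement or look input is locked per mode.
; At the spline's end it blends back and can destroy itself.
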(event OnActorBeginOverlap(TriggerBox)
  (params (OverlappedActor :type Actor%20Object%20Reference) (OtherActor :type Actor%20Object%20Reference))
  ;[1 1 1] Start Camera
  (if (== OtherActor (Game|Player|GetPlayerPawn 0))
    (Utilities|StartCameraSpline)))

(event Custom|StartCameraEvent
  ;[1 1 1] Start Camera
  (Utilities|StartCameraSpline))

(event Custom|SetCableCamera
  (bind _cablespline (Variables|SplineCable|GetCableSpline))
  ;[1 1 1] Set cable camera in right spot
  (if (and (Variables|Default|GetUseCableSpline?) (Utilities|IsValid _cablespline))
    (Transformation|SetRelativeTransform (Variables|Transformation|GetRootComponent self) (Math|Transform|MakeTransform (Transformation|GetWorldLocation (Variables|/Game/LevelDesign/LevelBlueprints/BP_SplineCable.BP_SplineCable_C|GetSpline _cablespline)) (Math|Rotator|MakeRotator 0.0 0.0 (.yaw (.rotation (Spline|GetTransformatDistanceAlongSpline (Variables|/Game/LevelDesign/LevelBlueprints/BP_SplineCable.BP_SplineCable_C|GetSpline (Variables|SplineCable|GetCableSpline)) 0.0 "World" false)))) "1.000000,1.000000,1.000000") false false)
    (Utilities|FlowControl|Sequence
      (:then_0
        (Utilities|FlowControl|DoOnce false
          (:Completed
            (Transformation|AddLocalOffset (Variables|Default|GetCamera) (Variables|SplineCable|GetCableCameraOffset) false false)
            (Utilities|CableCameraRot))))
      (:then_1
        (Utilities|CableCameraRot)))))

(event EventBeginPlay
  ;[1 1 1] Begin play
  (CallFunction|SetCableCamera)
  (if (Variables|AutomaticCamera|GetOnGameStart?)
    (Utilities|StartCameraSpline)))

(event EventTick
  (params (DeltaSeconds :type Float%20%28single-precision%29))
  (bind _returnvalue (Game|GetPlayerController 0))
  (bind _returnvalue_2 (Game|Player|GetPlayerPawn 0))
  (bind _spline (Variables|Default|GetSpline))
  (bind _camera (Variables|Default|GetCamera))
  (Variables|Default|SetDelta%20Seconds DeltaSeconds)
  (Utilities|FlowControl|Sequence
    (:then_0
      ;[1 1 1] Automatic Camera
      (if (and (Variables|Default|GetActive) (Variables|Default|GetAutomatic?))
        (CallFunction|AutomaticCamera)
        (Utilities|SplineFinished)))
    (:then_1
      ;[1 1 1] Cable Camera
      (if (and (Variables|Default|GetActive) (Variables|Default|GetUseCableSpline?))
        (Utilities|FlowControl|Sequence
          (:then_0
            (Utilities|FlowControl|DoOnce false :!label _label
              (:Completed
                (Rendering|SetVisibility (Variables|Default|GetSpark) true false))))
          (:then_1
            (CallFunction|SplineCableCamera)
            (Utilities|SplineFinished)
            (Utilities|FlowControl|Sequence
              (:then_0
                (goto _label Reset))
              (:then_1
                (Utilities|FlowControl|Delay 1.0)
                (CallFunction|SetCableCamera)))))))
    (:then_2
      ;[1 1 1] Player follow Camera
      (if (and (Variables|Default|GetActive) (Variables|Default|GetFollowPlayer?))
        (Utilities|FlowControl|Sequence
          (:then_0
            (Utilities|FlowControl|DoOnce false :!label _label_2
              (:Completed
                (Input|SetIgnoreLookInput (Game|GetPlayerController 0) true)
                (goto _label_3 Reset))))
          (:then_1
            (CallFunction|SplinePlayerCamera)
            (Utilities|SplineFinished)
            (Input|SetIgnoreLookInput (Game|GetPlayerController 0) false)
            (Utilities|ResetcameraRot)
            (goto _label_2 Reset))
          (:then_2
            (Utilities|FlowControl|DoOnce false :!label _label_3
              (:Completed
                (if (> (Variables|Default|GetDistanceAlongSpline) (/ (Spline|GetSplineLength (Variables|Default|GetSpline)) 2.0))
                  (Variables|PlayerFollowCamera|SetPlayerFollowCamOffset (Variables|PlayerFollowCamera|GetCameraOffset))
                  (Transformation|SetWorldRotation _camera (Math|Rotator|FindLookatRotation (Transformation|GetWorldLocation (Variables|Default|GetCamera)) (Transformation|GetWorldLocation (Variables|Default|GetSpline))) false false)
                  (else
                    (Variables|PlayerFollowCamera|SetPlayerFollowCamOffset (* (Variables|PlayerFollowCamera|GetCameraOffset) "(X=-1.000000,Y=0.000000)"))
                    (Transformation|SetWorldRotation _camera (Math|Rotator|FindLookatRotation (Transformation|GetWorldLocation (Variables|Default|GetCamera)) (Spline|GetLocationatSplinePoint _spline (Spline|GetNumberOfSplinePoints _spline) "World")) false false)))))))))
    (:then_3
      ;[1 1 1] Disable movement when camera is active
      (if (and (Variables|Default|GetActive) (not (Variables|Default|GetFollowPlayer?)))
        (Utilities|FlowControl|DoOnce false :!label _label_4
          (:Completed
            (Input|DisableInput _returnvalue_2 _returnvalue)
            (goto _label_5 Reset)))
        (else
          (Utilities|FlowControl|DoOnce false :!label _label_5
            (:Completed
              (Input|EnableInput _returnvalue_2 _returnvalue)
              (goto _label_4 Reset))))))))

(event Input|KeyboardEvents|1
  (params (Key :type Key%20Structure :default "None"))
  ;[1 1 1] Cancel camera
  (:Pressed
    (Utilities|ReturntoPlayer)))

(fn ConstructionScript)

(fn AutomaticCamera
  (bind _camera (Variables|Default|GetCamera))
  (Variables|Default|SetDistanceAlongSpline (+ (* (Variables|Default|GetDelta%20Seconds) (Variables|AutomaticCamera|GetSpeed)) (Variables|Default|GetDistanceAlongSpline)))
  (Variables|AutomaticCamera|SetSpeed (* (Variables|AutomaticCamera|GetBaseSpeed) (/ (Math|Curves|GetFloatValue (Variables|Default|GetSpeedCurve) (* (/ (Variables|Default|GetDistanceAlongSpline) (Spline|GetSplineLength (Variables|Default|GetSpline))) 1e+02)) 1e+02)))
  (if (Variables|AutomaticCamera|GetFreezeRotation?)
    (Transformation|SetRelativeTransform _camera (Math|Transform|MakeTransform (.location (Spline|GetTransformatDistanceAlongSpline (Variables|Default|GetSpline) (Variables|Default|GetDistanceAlongSpline) "Local" false)) "0, 0, 0" "1.000000,1.000000,1.000000") false false)
    (elif (Variables|AutomaticCamera|GetUseLookAtSpline?)
      (Transformation|SetRelativeTransform _camera (Math|Transform|MakeTransform (.location (Spline|GetTransformatDistanceAlongSpline (Variables|Default|GetSpline) (Variables|Default|GetDistanceAlongSpline) "Local" false)) (Math|Rotator|FindLookatRotation (Transformation|GetWorldLocation (Variables|Default|GetCamera)) (.location (Spline|GetTransformatDistanceAlongSpline (Variables|/Game/LevelDesign/LevelBlueprints/BP_Spline.BP_Spline_C|GetSpline (Variables|AutomaticCamera|GetLookAtSpline)) (* (Variables|Default|GetDistanceAlongSpline) (/ (Spline|GetSplineLength (Variables|/Game/LevelDesign/LevelBlueprints/BP_Spline.BP_Spline_C|GetSpline (Variables|AutomaticCamera|GetLookAtSpline))) (Spline|GetSplineLength (Variables|Default|GetSpline)))) "World" false))) "1.000000,1.000000,1.000000") false false)
      (else
        (Transformation|SetRelativeTransform _camera (Math|Transform|MakeTransform (.location (Spline|GetTransformatDistanceAlongSpline (Variables|Default|GetSpline) (Variables|Default|GetDistanceAlongSpline) "Local" false)) (.rotation (Spline|GetTransformatDistanceAlongSpline (Variables|Default|GetSpline) (Variables|Default|GetDistanceAlongSpline) "Local" false)) "1.000000,1.000000,1.000000") false false)))))

(fn SplineCableCamera
  (Variables|Default|SetDistanceAlongSpline (+ (* (Variables|Default|GetDelta%20Seconds) (Variables|SplineCable|GetCableSpeed)) (Variables|Default|GetDistanceAlongSpline)))
  (Transformation|SetRelativeTransform (Variables|Transformation|GetRootComponent self) (Math|Transform|MakeTransform (.location (Spline|GetTransformatDistanceAlongSpline (Variables|/Game/LevelDesign/LevelBlueprints/BP_SplineCable.BP_SplineCable_C|GetSpline (Variables|SplineCable|GetCableSpline)) (Variables|Default|GetDistanceAlongSpline) "World" false)) (Math|Rotator|MakeRotator 0.0 0.0 (.yaw (.rotation (Spline|GetTransformatDistanceAlongSpline (Variables|/Game/LevelDesign/LevelBlueprints/BP_SplineCable.BP_SplineCable_C|GetSpline (Variables|SplineCable|GetCableSpline)) (Variables|Default|GetDistanceAlongSpline) "World" false)))) "1.000000,1.000000,1.000000") false false)
  (Variables|SplineCable|SetCableSpeed (* (Variables|SplineCable|GetBaseCableSpeed) (/ (Math|Curves|GetFloatValue (Variables|Default|GetSpeedCurve) (* (/ (Variables|Default|GetDistanceAlongSpline) (Spline|GetSplineLength (Variables|/Game/LevelDesign/LevelBlueprints/BP_SplineCable.BP_SplineCable_C|GetSpline (Variables|SplineCable|GetCableSpline)))) 1e+02)) 1e+02)))
  (Development|PrintString (Utilities|String|ToString(Float) (/ (Math|Curves|GetFloatValue (Variables|Default|GetSpeedCurve) (* (/ (Variables|Default|GetDistanceAlongSpline) (Spline|GetSplineLength (Variables|/Game/LevelDesign/LevelBlueprints/BP_SplineCable.BP_SplineCable_C|GetSpline (Variables|SplineCable|GetCableSpline)))) 1e+02)) 1e+02)))
  (Utilities|CableCameraRot))

(fn SplinePlayerCamera
  (bind _playerfollowcamoffset (Variables|PlayerFollowCamera|GetPlayerFollowCamOffset))
  (bind _spline (Variables|Default|GetSpline))
  (Variables|Default|SetDistanceAlongSpline (Class|SplineComponent|GetDistanceAlongSplineatLocation (Variables|Default|GetSpline) (Transformation|GetWorldLocation (Variables|/Script/Engine.Character|GetCapsuleComponent (Game|GetPlayerCharacter 0))) "World"))
  (Transformation|SetWorldLocation (Variables|Default|GetCamera) (+ (.location (Spline|GetTransformatDistanceAlongSpline _spline (Variables|Default|GetDistanceAlongSpline) "World" false)) (* (Math|Vector|GetForwardVector _spline) (Math|Vector|MakeVector (.x _playerfollowcamoffset) (.x _playerfollowcamoffset) (.y _playerfollowcamoffset)))) false false))