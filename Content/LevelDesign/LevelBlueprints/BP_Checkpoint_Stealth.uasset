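; Checkpoint actor for the BP_Stealth pawn that marks itself active on overlap and serves as a respawn location.
; When usable, an overlap disables and hides every listed checkpoint with lower priority, then sets this one active and turns its cube green.
; Respawn teleports the passed BP_Stealth actor to the trigger box's location.
; The construction script colors the debug cube green or blue from the Active flag.
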(event OnComponentBeginOverlap(Box)
  (params (OverlappedComponent :type Primitive%20Component%20Object%20Reference) (OtherActor :type Actor%20Object%20Reference) (OtherComp :type Primitive%20Component%20Object%20Reference) (OtherBodyIndex :type Integer) (bFromSweep :type Boolean) (SweepResult :type Hit%20Result%20Structure%20%28by%20ref%29))
  (Utilities|Casting|CastToBP_Stealth OtherActor)
  (if (Variables|Default|GetCanBeUsed)
    (for _array_element (Variables|Default|GetCheckpoints)
      (if (not (>= (Variables|/Game/LevelDesign/LevelBlueprints/BP_Checkpoint.BP_Checkpoint_C|GetCheckpointPriority _array_element) (Variables|Default|GetCheckpointPriority)))
        (Variables|/Game/LevelDesign/LevelBlueprints/BP_Checkpoint.BP_Checkpoint_C|SetCanBeUsed _array_element false)
        (Rendering|SetVisibility (Variables|/Game/LevelDesign/LevelBlueprints/BP_Checkpoint.BP_Checkpoint_C|GetCube _array_element) false false)
        (Variables|/Game/LevelDesign/LevelBlueprints/BP_Checkpoint.BP_Checkpoint_C|SetActive _array_element false)))
    (Variables|Default|SetActive true)
    (Rendering|Material|SetMaterial (Variables|Default|GetCube) 0 "/Game/LevelDesign/BlockingStarterPack/Materials/Editor/MI_DevTriggerViewGreen.MI_DevTriggerViewGreen")))

(event EventBeginPlay
  (|CallParentFunction))

(event EventRespawn
  (params (RespawnActors :type Actor%20Object%20Reference))
  (bind _asbp_stealth (Utilities|Casting|CastToBP_Stealth RespawnActors))
  (Transformation|SetWorldLocation (Variables|/Script/Engine.Actor|GetRootComponent _asbp_stealth) (Transformation|GetWorldLocation (Variables|Default|GetBox)) false false))

(fn ConstructionScript
  (bind _cube (Variables|Default|GetCube))
  (if (Variables|Default|GetActive)
    (Rendering|Material|SetMaterial _cube 0 "/Game/LevelDesign/BlockingStarterPack/Materials/Editor/MI_DevTriggerViewGreen.MI_DevTriggerViewGreen")
    (else
      (Rendering|Material|SetMaterial _cube 0 "/Game/LevelDesign/BlockingStarterPack/Materials/Editor/MI_DevTriggerViewBlue.MI_DevTriggerViewBlue"))))