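; BP_LaserButton is a floor button that activates linked logic through ACExternal when a permitted actor steps on its Box trigger.
; WhoCanWalkOnIt allows any actor, only BP_Platformer or only BP_Stealth.
; Pressing plays a sound and lowers the Button mesh; unless OneTimeButton is set, emptying OverlappingActors reverses this and deactivates.
; Actors are only recorded while the button is inactive, so later arrivals do not hold it down.
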(event OnComponentBeginOverlap(Box)
  (params (OverlappedComponent :type Primitive%20Component%20Object%20Reference) (OtherActor :type Actor%20Object%20Reference) (OtherComp :type Primitive%20Component%20Object%20Reference) (OtherBodyIndex :type Integer) (bFromSweep :type Boolean) (SweepResult :type Hit%20Result%20Structure%20%28by%20ref%29))
  (bind _overlappingactors (Variables|Default|GetOverlappingActors))
  (if (not (Variables|Default|GetActive))
    (switch int (Variables|PlayerSettings|GetWho%20Can%20Walk%20On%20It?)
      (:1
        _)
      (:2
        (Utilities|Casting|CastToBP_Platformer OtherActor))
      (:3
        (Utilities|Casting|CastToBP_Stealth OtherActor)))
    (Utilities|Array|Add _overlappingactors OtherActor)
    (if (>= (Utilities|Array|Length _overlappingactors) 1)
      (Audio|PlaySoundatLocation "/Game/Audio/SFX/SFX_20241129/Fuse_-_sfx_-_ButtonOn.Fuse_-_sfx_-_ButtonOn" (Transformation|GetWorldLocation (Variables|Default|GetBase)) "0, 0, 0" 1.0 1.0 0.0 0 0 0 0)
      (Transformation|SetWorldLocation (Variables|Default|GetButton) (- (Transformation|GetWorldLocation (Variables|Default|GetBase)) "0.000000,0.000000,5.000000") false false)
      (Default|ActivateThis (Variables|Default|GetAC_External))
      (Variables|Default|SetActive true))))

(event OnComponentEndOverlap(Box)
  (params (OverlappedComponent :type Primitive%20Component%20Object%20Reference) (OtherActor :type Actor%20Object%20Reference) (OtherComp :type Primitive%20Component%20Object%20Reference) (OtherBodyIndex :type Integer))
  (bind _overlappingactors (Variables|Default|GetOverlappingActors))
  (if (and (Variables|Default|GetActive) (not (Variables|PlayerSettings|GetOne%20Time%20Button?)))
    (Utilities|Array|RemoveItem _overlappingactors OtherActor)
    (if (<= (Utilities|Array|Length _overlappingactors) 0)
      (Audio|PlaySoundatLocation "/Game/Audio/SFX/SFX_20241129/Fuse_-_sfx_-_ButtonOn.Fuse_-_sfx_-_ButtonOn" (Transformation|GetWorldLocation (Variables|Default|GetBase)) "0, 0, 0" 1.0 1.0 0.0 0 0 0 0)
      (Transformation|SetWorldLocation (Variables|Default|GetButton) (Variables|Default|GetBase%20Standard) false false)
      (Default|DeactivateThis (Variables|Default|GetAC_External))
      (Variables|Default|SetActive false))))

(event EventBeginPlay
  (Variables|Default|SetBase%20Standard (Transformation|GetWorldLocation (Variables|Default|GetBase))))

(fn ConstructionScript)