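; BP_PuzzleRock is a pushable puzzle rock that slides one step along world X or Y when hit by a BP_Stealth character.
; The dominant axis of their relative position sets the direction away from the character, and MovingPower scales the step.
; Box traces sized from the mesh bounds block moves into obstacles or past floor edges.
; PushingTimeline lerps the actor to the target, with IsMoving ignoring hits meanwhile.
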(event Collision|EventHit
  (params (MyComp :type Primitive%20Component%20Object%20Reference) (Other :type Actor%20Object%20Reference) (OtherComp :type Primitive%20Component%20Object%20Reference) (bSelfMoved :type Boolean) (HitLocation :type Vector :default "0, 0, 0") (HitNormal :type Vector :default "0, 0, 0") (NormalImpulse :type Vector :default "0, 0, 0") (Hit :type Hit%20Result%20Structure%20%28by%20ref%29))
  (bind _staticmesh (Variables|Default|GetStaticMesh))
  (bind _bounds_extra_area (Variables|Default|GetBounds%20Extra%20Area))
  (bind _staticmesh_2 (Variables|Default|GetStaticMesh))
  (bind _boxextent (Collision|GetComponentBounds _staticmesh_2))
  (bind _boxextent_2 (Collision|GetComponentBounds _staticmesh))
  (if (not (Variables|Default|GetisMoving))
    ;[1 1 1] Check if actor is Stealth Character
    (Utilities|Casting|CastToBP_Stealth Other)
    (Variables|Default|SetisMoving true)
    (Variables|Default|SetRelativePosition (- (Transformation|GetActorLocation) (Transformation|GetActorLocation Other)))
    (if (> (.x (Math|Vector|VectorGetAbs (Variables|Default|GetRelativePosition))) (.y (Math|Vector|VectorGetAbs (Variables|Default|GetRelativePosition))))
      (bind _output_get (Variables|Default|SetNewPosition (+ (Transformation|GetActorLocation) (Math|Vector|MakeVector (* (.x (Class|KismetMathLibrary|VectorGetSignVector (Math|Vector|MakeVector (.x (Variables|Default|GetRelativePosition)) 0.0 0.0))) (Variables|Default|GetMovingPower)) 0.0 0.0))))
      (Variables|Default|SetIs%20There%20An%20Edge%20Here? (+ _output_get (Math|Vector|MakeVector (* (* (.x (Class|KismetMathLibrary|VectorGetSignVector (Math|Vector|MakeVector (.x (Variables|Default|GetRelativePosition)) 0.0 0.0))) (Variables|Default|GetMovingPower)) 2.0) 0.0 0.0)))
      (else
        (bind _output_get_2 (Variables|Default|SetNewPosition (+ (Transformation|GetActorLocation) (Math|Vector|MakeVector 0.0 (* (.y (Class|KismetMathLibrary|VectorGetSignVector (Math|Vector|MakeVector 0.0 (.y (Variables|Default|GetRelativePosition)) 0.0))) (Variables|Default|GetMovingPower)) 0.0))))
        (Variables|Default|SetIs%20There%20An%20Edge%20Here? (+ _output_get_2 (Math|Vector|MakeVector 0.0 (* (* (.y (Class|KismetMathLibrary|VectorGetSignVector (Math|Vector|MakeVector 0.0 (.y (Variables|Default|GetRelativePosition)) 0.0))) (Variables|Default|GetMovingPower)) 2.0) 0.0)))))
    (bind _returnvalue (Collision|BoxTraceByChannel (Transformation|GetActorLocation) (Variables|Default|GetNewPosition) (Math|Vector|MakeVector (+ (.x _boxextent) _bounds_extra_area) (+ (.y _boxextent) _bounds_extra_area) (.z _boxextent)) "0, 0, 0" "TraceTypeQuery1" false 0 "None"))
    (if _returnvalue
      (Variables|Default|SetisMoving false)
      (else
        ;[1 1 1] Checking so the box won't be hanging outside an edge
        (bind _returnvalue_2 (Collision|BoxTraceByChannel (Variables|Default|GetIs%20There%20An%20Edge%20Here?) (Variables|Default|GetIs%20There%20An%20Edge%20Here?) (Math|Vector|MakeVector (.x _boxextent_2) (.y _boxextent_2) (+ (.z _boxextent_2) (Variables|Default|GetFloor%20Check))) "0, 0, 0" "TraceTypeQuery1" false 0 "None"))
        (if _returnvalue_2
          ;[1 1 1] Start the Moving
          (bind _moving_rock (Timeline|Pushing%20Timeline PlayFromStart)
            (:Update
              (Transformation|SetActorLocation (Math|Vector|Lerp(Vector) (Transformation|GetActorLocation) (Variables|Default|GetNewPosition) _moving_rock) false false))
            (:Finished
              (Variables|Default|SetisMoving false)))
          (else
            (Variables|Default|SetisMoving false)))))))

(fn ConstructionScript)

(fn CheckifHangingOutAnEdge)