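; BP_Laser is a laser beam actor that line-traces forward every tick and stretches its mesh to the blocking hit or full range.
; Hit actors' AC_Handler components, used for bouncing, get start, update and stop messages by comparing hit sets between frames, while AC_External components receive hits for destroying doors or enemies.
; Handlers owning earlier lasers in the chain are skipped to prevent loops.
; It creates a dynamic material, but the color override call is disconnected.
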(event EventBeginPlay
  (bind _returnvalue (Rendering|Material|CreateDynamicMaterialInstance "/Game/Lasers/Materials/M_Laser.M_Laser" "None" "None" :!class /Script/Engine.KismetMaterialLibrary))
  (bind _output_get (Variables|Default|SetMaterial%20Instance _returnvalue))
  (Rendering|Material|SetMaterial (Variables|Default|GetStaticMesh) 0 _output_get))

(event EventTick
  (params (DeltaSeconds :type Float%20%28single-precision%29))
  (bind _returnvalue (Transformation|GetActorLocation))
  (bind (_outhits _returnvalue_2) (Collision|MultiLineTraceByChannel _returnvalue (+ _returnvalue (* (Transformation|GetActorForwardVector) (Variables|Exposed|GetRange))) "TraceTypeQuery3" true (Variables|Exposed|GetActors%20To%20Ignore) "None"))
  (if _returnvalue_2
    (for _array_element _outhits
      (Utilities|FlowControl|Sequence
        (:then_0
          (if (.bBlockingHit (Collision|BreakHitResult _array_element))
            (CallFunction|UpdateLength (.Distance (Collision|BreakHitResult _array_element)))))
        (:then_1
          (CallFunction|HandleHitActors _array_element))))
    (else
      (CallFunction|UpdateLength (Variables|Exposed|GetRange))))
  (bind _result (Utilities|Set|Difference (Variables|Default|GetPreviously%20Hit%20Handlers) (Variables|Default|GetCurrent%20Hit%20Handles)))
  (bind _result_2 (Utilities|Set|ToArray _result))
  (for _array_element_2 _result_2
    (Class|BPILasers|LaserStopHitting(Message) _array_element_2 self)
    (Utilities|Map|Remove (Variables|Default|GetHitting%20Handlers) _array_element_2))
  (Variables|Default|SetPreviously%20Hit%20Handlers (Variables|Default|GetCurrent%20Hit%20Handles))
  (Utilities|Set|Clear (Variables|Default|GetCurrent%20Hit%20Handles)))

(event EventLaserStopHitting
  (params (Input :type BP%20Laser%20Object%20Reference))
  (Utilities|FlowControl|Sequence
    (:then_0
      (bind _result (Utilities|Set|ToArray (Variables|Default|GetPreviously%20Hit%20Handlers)))
      (for _array_element _result
        (Class|BPILasers|LaserStopHitting(Message) _array_element self)))
    (:then_1
      (Actor|DestroyActor))))

(fn ConstructionScript)

(fn ChangeLaserColor
  (params (Value :type Linear%20Color%20Structure))
  (Rendering|Material|SetVectorParameterValue (Variables|Default|GetMaterial%20Instance) "Color" Value :!class /Script/Engine.MaterialInstanceDynamic))

(fn UpdateLength
  (params (InputPin :type Float%20%28single-precision%29))
  (bind _beam_width (Variables|Exposed|GetBeam%20Width))
  (if (not (Math|Float|NearlyEqual(Float) InputPin (Variables|Default|GetPrevious%20Length) 2.0))
    (bind _output_get (Variables|Default|SetPrevious%20Length InputPin))
    (Transformation|SetWorldScale3D (Variables|Default|GetStaticMesh) (Math|Vector|MakeVector _beam_width _beam_width (/ _output_get 1e+02)))))

(fn HandleHitActors
  (params (InputPin :type Hit%20Result%20Structure))
  (bind _hitactor (Collision|BreakHitResult InputPin))
  (bind _returnvalue (Actor|GetComponentbyClass _hitactor "/Game/Lasers/Blueprints/BuildingBlocks/AC_External.AC_External_C"))
  (bind _returnvalue_2 (Actor|GetComponentbyClass _hitactor "/Game/Lasers/Blueprints/BuildingBlocks/AC_Handler.AC_Handler_C"))
  ;[1 1 1] For Bouncing Laser
  (Utilities|IsValid _returnvalue_2
    (:Is%20Valid
      (LocalVariables|SetL_Handler _returnvalue_2)
      (if (CallFunction|IsNotonPath (LocalVariables|GetL_Handler))
        (Utilities|Map|Add (Variables|Default|GetHitting%20Handlers) (LocalVariables|GetL_Handler) InputPin)
        (if (Utilities|Set|Contains (Variables|Default|GetPreviously%20Hit%20Handlers) (LocalVariables|GetL_Handler))
          (Default|LaserUpdateHitting (LocalVariables|GetL_Handler) self InputPin)
          (else
            (Class|BPILasers|LaserStartHitting(Message) (LocalVariables|GetL_Handler) self InputPin)))
        (Utilities|Set|Add (Variables|Default|GetCurrent%20Hit%20Handles) (LocalVariables|GetL_Handler))))
    (:Is%20Not%20Valid
      ;[1 1 1] For Destroying Doors/Enemies
      (Utilities|IsValid _returnvalue
        (:Is%20Valid
          (Class|BPILasers|LaserStartHitting(Message) _returnvalue self InputPin))))))

(fn IsNotonPath
  (params (InputHandler :type AC%20Handler%20Object%20Reference))
  (if (Utilities|Array|IsNotEmpty (Variables|Exposed|GetPrevious%20Lasers))
    (for _array_element (Variables|Exposed|GetPrevious%20Lasers)
      (bind _output_get (LocalVariables|SetL_CurrentLaser _array_element))
      (if (== (Variables|BP_Laser_C|GetOwning%20Handler _output_get) InputHandler)
        (return false)
        (elif (not true)
          (return false))))
    (return true)
    (else
      (return true))))

(fn GetHitbyHandler
  (params (Key :type AC%20Handler%20Object%20Reference%20%28by%20ref%29))
  (bind _hitting_handlers (Variables|Default|GetHitting%20Handlers))
  (bind (_value _returnvalue) (Utilities|Map|Find _hitting_handlers Key))
  (return _value _returnvalue))