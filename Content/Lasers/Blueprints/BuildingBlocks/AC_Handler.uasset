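; Laser-system handler component that receives laser hit events and relays them to the owner's other components implementing BPI_Lasers.
; On BeginPlay it caches those components, sets static mesh responses on the laser trace channel to block or overlap, and optionally sends stop-hit to emitters for inverted setups.
; Start and stop events update a queue of incoming lasers and forward only while unlocked.
; Update events always pass through, bypassing the lock.
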(event EventBeginPlay
  (Utilities|FlowControl|Sequence
    (:then_0
      (bind _output_get (Variables|Default|SetLinked%20Components (Class|Actor|GetComponentsbyInterface (Components|GetOwner) "/Game/Lasers/Blueprints/BuildingBlocks/BPI_Lasers.BPI_Lasers_C")))
      (Utilities|Array|RemoveItem _output_get self)
      (for _array_element (Actor|GetComponentsByClass (Components|GetOwner) "/Script/Engine.StaticMeshComponent")
        (Collision|SetCollisionResponsetoChannel _array_element "ECC_GameTraceChannel1" (select (Variables|Conditions|GetisBlocking) "ECR_Block" "ECR_Overlap"))))
    (:then_1
      (if (Variables|Conditions|GetInvert%20System)
        (for _array_element_2 (Actor|GetComponentsByClass (Components|GetOwner) "/Game/Lasers/Blueprints/BuildingBlocks/SC_Emitter.SC_Emitter_C")
          (Default|LaserStopHitting _array_element_2))))))

(event EventLaserUpdateHitting
  (params (Input :type A%20Laser%20Object%20Reference) (Hit%20Info :type Hit%20Result%20Structure))
  (bind _array_element (Utilities|ForEachComponent)
    (:LoopBody
      (Class|BPILasers|LaserUpdateHitting(Message) _array_element Input Hit%20Info))))

(event EventLaserStartHitting
  (params (Input :type A%20Laser%20Object%20Reference) (Hit%20Info :type Hit%20Result%20Structure))
  (CallFunction|LaserAdded Input)
  (Utilities|IsNotLocked
    (:Not%20Locked
      (bind _array_element (Utilities|ForEachComponent)
        (:LoopBody
          (Class|BPILasers|LaserStartHitting(Message) _array_element Input Hit%20Info))))))

(event EventLaserStopHitting
  (params (Input :type A%20Laser%20Object%20Reference))
  (CallFunction|LaserRemoved Input)
  (Utilities|IsNotLocked
    (:Not%20Locked
      (bind _array_element (Utilities|ForEachComponent)
        (:LoopBody
          (Class|BPILasers|LaserStopHitting(Message) _array_element Input))))))

(fn LaserAdded
  (params (NewItem :type A%20Laser%20Object%20Reference%20%28by%20ref%29))
  (Utilities|Array|AddUnique (Variables|Default|GetLaser%20in%20Queue) NewItem))

(fn LaserRemoved
  (params (NewItem :type A%20Laser%20Object%20Reference%20%28by%20ref%29))
  (Utilities|Array|RemoveItem (Variables|Default|GetLaser%20in%20Queue) NewItem))