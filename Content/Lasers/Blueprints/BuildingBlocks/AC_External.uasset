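; Actor component that reacts to a laser hit by animating a material effect from the impact point, then destroying its owner or respawning it if it is the player.
; The first hit creates a dynamic material instance on the hit component and opens a gated Tick that grows the Scale parameter.
; The impact is stored in actor-local space so Location follows movement.
; After a delay the gate closes; player respawns go through BP_DeathArea and reset the effect.
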(event EventTick
  (params (DeltaSeconds :type Float%20%28single-precision%29))
  (bind _reference (Variables|Default|GetReference))
  (Utilities|FlowControl|Gate true
    (:Exit
      (bind _output_get (Variables|Default|SetTime (+ (Variables|Default|GetTime) (* DeltaSeconds (Variables|Variables|GetSpeedOfAnimation)))))
      (Rendering|Material|SetVectorParameterValue _reference "Scale" (Utilities|Struct|MakeLinearColor _output_get _output_get _output_get 1.0) :!class /Script/Engine.MaterialInstanceDynamic)
      (Rendering|Material|SetVectorParameterValue _reference "Location" (Math|Conversions|ToLinearColor(Vector) (Math|Transform|TransformLocation (Transformation|GetActorTransform (.HitActor (Collision|BreakHitResult (stale EventLaserStartHitting Hit%20Info)))) (Variables|Default|GetImpact%20Point))) :!class /Script/Engine.MaterialInstanceDynamic))))

(event EventLaserStartHitting
  (params (Input :type BP%20Laser%20Object%20Reference) (Hit%20Info :type Hit%20Result%20Structure))
  (bind (_bblockinghit _binitialoverlap _time _distance _location _impactpoint _normal _impactnormal _physmat _hitactor _hitcomponent) (Collision|BreakHitResult Hit%20Info))
  (bind _returnvalue (Transformation|GetActorTransform _hitactor))
  (Utilities|IsValid _hitcomponent
    (:Is%20Valid
      (if (not (Variables|Default|GetDoOnce))
        (Variables|Default|SetDoOnce true)
        (Variables|Default|SetImpact%20Point (Math|Transform|InverseTransformLocation _returnvalue _impactpoint))
        (bind _returnvalue_2 (Rendering|Material|CreateDynamicMaterialInstance _hitcomponent 0 (Rendering|Material|GetMaterial _hitcomponent 0) "None" :!class /Script/Engine.PrimitiveComponent))
        (bind _output_get (Variables|Default|SetReference _returnvalue_2))
        (Rendering|Material|SetVectorParameterValue _output_get "Location" (Math|Conversions|ToLinearColor(Vector) _impactpoint) :!class /Script/Engine.MaterialInstanceDynamic)
        (Variables|Default|SetTime 0.0)
        (Utilities|FlowControl|Sequence
          (:then_0
            (Utilities|FlowControl|Gate true) ; enters at Open
          )
          (:then_1
            (Utilities|FlowControl|Delay (Variables|Variables|GetTime%20Until%20Destruction))
            (Utilities|FlowControl|Sequence
              (:then_0
                (Utilities|FlowControl|Gate true) ; enters at Close
              )
              (:then_1
                (CallFunction|DestroyorRespawn)))))))))

(fn DestroyorRespawn
  (if (Variables|Variables|GetIsPlayer?)
    (bind _returnvalue (Actor|GetActorOfClass "/Game/LevelDesign/LevelBlueprints/BP_DeathArea.BP_DeathArea_C"))
    (Default|PlayerRespawn _returnvalue (Components|GetOwner))
    (Variables|Default|SetDoOnce false)
    (Rendering|Material|SetVectorParameterValue (Variables|Default|GetReference) "Scale" (Utilities|Struct|MakeLinearColor 0.0 0.0 0.0 1.0) :!class /Script/Engine.MaterialInstanceDynamic)
    (else
      (Actor|DestroyActor (Components|GetOwner)))))