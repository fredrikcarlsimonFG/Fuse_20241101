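; SC_Emitter is a scene component that emits an A_Laser from its transform as a building block of the laser system.
; It caches the owner's AC_Handler, and hit start/stop events activate or deactivate the beam, swapped when the system is inverted.
; Activation spawns and attaches a laser that ignores the owner, passing it the filtered lasers and the last one's color.
; Deactivation tells the attached laser to stop hitting.
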(event EventBeginPlay
  (bind _returnvalue (Components|GetOwner))
  (bind _returnvalue_2 (Actor|GetComponentbyClass _returnvalue "/Game/Lasers/Blueprints/BuildingBlocks/AC_Handler.AC_Handler_C"))
  (Utilities|IsValid _returnvalue_2
    (:Is%20Valid
      (Variables|Default|SetOwning%20Handler _returnvalue_2))))

(event EventLaserStartHitting
  (params (Input :type A%20Laser%20Object%20Reference) (Hit%20Info :type Hit%20Result%20Structure))
  (if (Utilities|IsSystemInverted)
    (CallFunction|DeactivateLaser)
    (else
      (CallFunction|ActivateLaser))))

(event EventLaserStopHitting
  (params (Input :type A%20Laser%20Object%20Reference))
  (if (Utilities|IsSystemInverted)
    (CallFunction|ActivateLaser)
    (else
      (CallFunction|DeactivateLaser))))

(fn ActivateLaser
  (bind _outputpin (Utilities|GetFilteredLasers))
  (if (Utilities|Array|IsNotEmpty _outputpin)
    (Variables|Default|SetCurent%20Color (Variables|/Game/Lasers/Blueprints/BuildingBlocks/A_Laser.A_Laser_C|GetColor%20Override (Utilities|Array|Get(acopy) _outputpin (Utilities|Array|LastIndex _outputpin)))))
  (bind _returnvalue (Game|SpawnActorfromClass "/Game/Lasers/Blueprints/BuildingBlocks/A_Laser.A_Laser_C" (Transformation|GetWorldTransform) "Undefined" "MultiplyWithRoot" 0 (Variables|Default|GetCurent%20Color) (Variables|Default|GetMax%20Range) (Utilities|GetFilteredLasers) (Variables|Default|GetOwning%20Handler) (Utilities|Array|MakeArray (Components|GetOwner)) 0))
  (bind _output_get (Variables|Default|SetAttached%20Laser _returnvalue))
  (Transformation|AttachComponentToComponent _output_get self "None" "KeepWorld" "KeepWorld" "KeepWorld" false))

(fn DeactivateLaser
  (bind _attached_laser (Variables|Default|GetAttached%20Laser)
    (:then
      (Default|LaserStopHitting _attached_laser))
    (:else)))